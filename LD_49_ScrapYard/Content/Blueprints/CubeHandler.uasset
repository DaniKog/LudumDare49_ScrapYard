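; Handler actor for a cube-stacking game that spawns a swinging cube and drops it on key press.
; Each Tick applies sine-driven sway and swivel to the unreleased cube, with rope-cut audio on release and camera shake on impact.
; On landing it finds the highest cube, moves itself to an offset above it, then fires AddNewCube.
; That event spawns the next cube, using a random class from Game_Cube actors gathered at construction.
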(event Custom|OnCubeLanded
  (EventDispatchers|UnbindallEventsfromOnCubeLandeed (Variables|Default|GetCurrentCube))
  (Variables|Default|SetInitialCameraPosition (Transformation|GetActorLocation))
  (CallFunction|GetHighestCubeZ)
  (Variables|Default|SetMoveUp true))

(event Custom|CubeReleaseKeyPressed
  (bind _currentcube (Variables|Default|GetCurrentCube))
  (bind _releasesound (Variables|Default|GetReleaseSound))
  (if (Variables|Default|GetInGame)
    (bind _soundtoplay (CallFunction|GetRandomSound (Variables|Default|GetCutRopeSound)))
    (Audio|Components|Audio|SetSound _releasesound _soundtoplay)
    (Audio|Components|Audio|Play _releasesound 0.0)
    (Audio|Components|Audio|Stop (Variables|Default|GetHandlerAudio))
    (Default|ReleaseCube _currentcube)
    (Default|CallCubeReleased)
    (if (Variables|Default|GetInGame)
      (EventDispatchers|BindEventtoOnCubeLandeed _currentcube (delegate Custom|OnCubeLanded))
      (EventDispatchers|BindEventtoOnCubeHit _currentcube (delegate Custom|OnCubeHit))
      (Variables|Default|SetIdle_Movement_Cycle1 5.0)
      (Variables|Default|SetIdle_Movement_Cycle2 1e+01))))

(event Custom|OnCubeReadyToAdd
  (if (Variables|Default|GetInGame)
    (CallFunction|SetCurrentCubeInitalValues)))

(event Custom|OnCubeHit
  (Camera|PlayWorldCameraShake "/Game/Blueprints/InitCamShake.InitCamShake_C" (Transformation|GetActorLocation) 0.0 5e+02)
  (EventDispatchers|UnbindallEventsfromOnCubeHit (Variables|Default|GetCurrentCube))
  (Default|PlayHardImpactSound (Variables|Default|GetCurrentCube)))

(event EventBeginPlay
  (Input|EnableInput (Game|GetPlayerController 0))
  (EventDispatchers|BindEventtoAddNewCube (delegate Custom|OnCubeReadyToAdd)))

(event Collision|EventActorBeginOverlap
  (params (OtherActor :type Actor%20Object%20Reference)))

(event EventTick
  (params (DeltaSeconds :type Float%20%28single-precision%29))
  (CallFunction|IdleMoveCubeSin2 DeltaSeconds)
  (CallFunction|MoveCameraUp 3e+02 (Variables|Default|GetCamera%20movement%20Speed) DeltaSeconds))

(fn ConstructionScript
  (Variables|Default|SetIdle_Vec_Swivel_X (Math|Vector|RotateVectorAroundAxis "1.000000, 0, 0" (Variables|Default|GetIdle_Swivel_X) "0, 0,1.000000"))
  (Variables|Default|SetIdle_Vec_Swivel_Y (Math|Vector|RotateVectorAroundAxis "0,1.000000, 0" (Variables|Default|GetIdle_Swivel_Y) "0, 0,1.000000"))
  (bind _outactors (Actor|GetAllActorsOfClass "/Game/Blueprints/Game_Cube.Game_Cube_C"))
  (Variables|Default|SetGameCubes _outactors))

(fn IdleMoveCube
  (bind _currentcube (Variables|Default|GetCurrentCube))
  (bind _initalcubeposition (Variables|Default|GetInitalCubePosition))
  (bind _cube (Variables|/Game/Blueprints/Game_Cube.Game_Cube_C|GetCube _currentcube))
  (bind _returnvalue (Transformation|GetWorldLocation _cube))
  (bind _returnvalue_2 (- _initalcubeposition _returnvalue))
  (bind _z (Math|Vector|BreakVector _returnvalue_2))
  (Transformation|AddWorldOffset (Variables|/Game/Blueprints/Game_Cube.Game_Cube_C|GetCube _currentcube) (Math|Vector|MakeVector (Variables|Default|GetDirection_Speed_Y) 0.0 (Variables|Default|GetDirection_Speed_Z)) false false)
  (if (or (<= _z -3e+01) (>= _z 3e+01))
    (bind _result (Math|Float|NegateFloat (Variables|Default|GetDirection_Speed_Z))
      (:%20%20
        (Variables|Default|SetDirection_Speed_Z _result)))))

(fn IdleMoveCubeSin
  (bind _currentcube (Variables|Default|GetCurrentCube))
  (bind _currentcube_2 (Variables|Default|GetCurrentCube))
  (bind _initalcubeposition (Variables|Default|GetInitalCubePosition))
  (bind _initialrotation (Variables|Default|GetInitialRotation))
  (bind _cube (Variables|/Game/Blueprints/Game_Cube.Game_Cube_C|GetCube _currentcube_2))
  (bind _cube_2 (Variables|/Game/Blueprints/Game_Cube.Game_Cube_C|GetCube _currentcube))
  (bind _returnvalue (Transformation|GetWorldLocation _cube_2))
  (bind _returnvalue_2 (Transformation|GetWorldRotation _cube))
  (bind _returnvalue_3 (Math|Rotator|Delta(Rotator) _initialrotation _returnvalue_2))
  (bind _returnvalue_4 (- _initalcubeposition _returnvalue))
  (bind _roll (Math|Rotator|BreakRotator _returnvalue_3))
  (bind (_x _y _z) (Math|Vector|BreakVector _returnvalue_4))
  (bind _returnvalue_5 (* _y 1.449))
  (bind _returnvalue_6 (Math|Trig|Cos(Degrees) _returnvalue_5))
  (if (not (Variables|/Game/Blueprints/Game_Cube.Game_Cube_C|GetReleased _currentcube))
    (Transformation|AddWorldOffset (Variables|/Game/Blueprints/Game_Cube.Game_Cube_C|GetCube _currentcube) (Math|Vector|MakeVector 0.0 (* (Variables|Default|GetCurrentSinMulipler) (Variables|Default|GetDirection_Speed_Y)) (* (Variables|Default|GetCurrentSinMulipler) (Variables|Default|GetDirection_Speed_Z))) false false)
    (Transformation|AddLocalRotation _cube (Math|Rotator|MakeRotator (* (Variables|Default|GetYRoationSpeed) (Variables|Default|GetCurrentSinMulipler)) 0.0 0.0) false false)
    (if (or (<= _roll -18.0) (>= _roll 18.0))
      (bind _result (Math|Float|NegateFloat (Variables|Default|GetYRoationSpeed))
        (:%20%20
          _)))
    (Variables|Default|SetCurrentSinMulipler _returnvalue_6)
    (if (Math|Boolean|ORBoolean (<= _z -3e+01) (>= _z 3e+01) (Math|Float|NearlyEqual(Float) _returnvalue_6 1.0 0.0001))
      (bind _result_2 (Math|Float|NegateFloat (Variables|Default|GetDirection_Speed_Z))
        (:%20%20
          (Variables|Default|SetDirection_Speed_Z _result_2))))
    (if (or (<= _y -6e+01) (>= _y 6e+01))
      (bind _result_3 (Math|Float|NegateFloat (Variables|Default|GetDirection_Speed_Y))
        (:%20%20
          (Variables|Default|SetDirection_Speed_Y _result_3))))))

(fn SetCurrentCubeInitalValues
  (bind _gamecubes (Variables|Default|GetGameCubes))
  (bind _returnvalue (Game|SpawnActorfromClass (Utilities|GetClass (Utilities|Array|Get(acopy) _gamecubes (Math|Random|RandomInteger (Utilities|Array|Length _gamecubes)))) (Math|Transform|MakeTransform (+ (Transformation|GetActorLocation) "0,-50.000000, 0")) "Undefined" 0 0))
  (bind _output_get (Variables|Default|SetCurrentCube _returnvalue))
  (Variables|Default|SetInitalCubePosition (Transformation|GetActorLocation _output_get))
  (Variables|Default|SetInitialRotation (Transformation|GetActorRotation _output_get))
  (Variables|/Game/Blueprints/Game_Cube.Game_Cube_C|SetReleased _output_get false)
  (Audio|Components|Audio|Play (Variables|Default|GetHandlerAudio) 0.0))

(fn IdleMoveCubeSin2
  (params (DeltaTime :type Float%20%28single-precision%29))
  (bind _currentcube (Variables|Default|GetCurrentCube))
  (bind _idle_swiwelspeedmultiplayer (Variables|Default|GetIdle_SwiwelSpeedMultiplayer))
  (bind _idle_movement_speedmultipler (Variables|Default|GetIdle_Movement_SpeedMultipler))
  (bind _returnvalue (* DeltaTime _idle_swiwelspeedmultiplayer))
  (bind _returnvalue_2 (* DeltaTime _idle_movement_speedmultipler))
  (bind _cube (Variables|/Game/Blueprints/Game_Cube.Game_Cube_C|GetCube _currentcube))
  (bind _returnvalue_3 (* _returnvalue 3.6e+02))
  (bind _returnvalue_4 (* _returnvalue_2 3.6e+02))
  (if (Utilities|IsValid (Variables|Default|GetCurrentCube))
    (if (not (Variables|/Game/Blueprints/Game_Cube.Game_Cube_C|GetReleased (Variables|Default|GetCurrentCube)))
      (Variables|Default|SetIdle_CurrentSwiwel_X (Math|Float|%(Float) (+ (/ _returnvalue_3 (Variables|Default|GetIdle_Swivel_X)) (Variables|Default|GetIdle_CurrentSwiwel_X)) 3.6e+02))
      (Variables|Default|SetIdle_CurrentSwiwel_Y (Math|Float|%(Float) (+ (/ _returnvalue_3 (Variables|Default|GetIdle_Swivel_Y)) (Variables|Default|GetIdle_CurrentSwiwel_Y)) 3.6e+02))
      (Transformation|SetRelativeRotation (Variables|/Game/Blueprints/Game_Cube.Game_Cube_C|GetCube (Variables|Default|GetCurrentCube)) (Math|Rotator|MakeRotfromXY (Math|Vector|RotateVectorAroundAxis (Variables|Default|GetIdle_Vec_Swivel_X) (Variables|Default|GetIdle_CurrentSwiwel_X) "1.000000, 0, 0") (Math|Vector|RotateVectorAroundAxis (Variables|Default|GetIdle_Vec_Swivel_Y) (Variables|Default|GetIdle_CurrentSwiwel_Y) "0,1.000000, 0")) false false)
      (Utilities|FlowControl|Sequence
        (:then_0
          (Variables|Default|SetIdle_Movement_Cycle1 (Math|Float|%(Float) (+ (Variables|Default|GetIdle_Movement_Cycle1) (/ _returnvalue_4 (Variables|Default|GetIdle_Movement_Period1))) 3.6e+02)))
        (:then_1
          (Variables|Default|SetIdle_Movement_Cycle2 (Math|Float|%(Float) (+ (Variables|Default|GetIdle_Movement_Cycle2) (/ _returnvalue_4 (Variables|Default|GetIdle_Movement_Period2))) 3.6e+02)))
        (:then_2
          (Variables|Default|SetIdle_Movement_Cycle3 (Math|Float|%(Float) (+ (Variables|Default|GetIdle_Movement_Cycle3) (/ _returnvalue_4 (Variables|Default|GetIdle_Movement_Period3))) 3.6e+02)))
        (:then_3
          (Transformation|AddWorldOffset _cube (Math|Vector|MakeVector 0.0 (* (Variables|Default|GetIdle_Movement_Amplitude1_Y) (Math|Trig|Sin(Degrees) (Variables|Default|GetIdle_Movement_Cycle1))) (* (Variables|Default|GetIdle_Movement_Amplitude2_Z) (Math|Trig|Sin(Degrees) (Variables|Default|GetIdle_Movement_Cycle2)))) false false)
          (Class|KismetMathLibrary|VectorNormalize (Transformation|GetWorldLocation _cube) 0.0))))))

(fn MoveCameraUp
  (params (Offset%20Z :type Float%20%28single-precision%29) (MovementSpeed :type Float%20%28single-precision%29) (DeltaTime :type Float%20%28single-precision%29))
  (bind _returnvalue (* MovementSpeed DeltaTime))
  (bind _defaultsceneroot (Variables|Default|GetDefaultSceneRoot))
  (bind _highestcube_zvalue (Variables|Default|GetHighestCube_ZValue))
  (bind _returnvalue_2 (Transformation|GetWorldLocation _defaultsceneroot))
  (bind _returnvalue_3 (+ Offset%20Z _highestcube_zvalue))
  (bind _z (Math|Vector|BreakVector _returnvalue_2))
  (if (Variables|Default|GetMoveUp)
    (if (< _z _returnvalue_3)
      (Transformation|AddActorWorldOffset (Math|Vector|MakeVector 0.0 0.0 _returnvalue))
      (elif (> -3.0 (- _returnvalue_3 _z))
        (Transformation|AddActorWorldOffset (Math|Vector|MakeVector 0.0 0.0 (* _returnvalue -1.0)))
        (else
          (Variables|Default|SetMoveUp false)
          (Default|CallAddNewCube))))))

(fn GetHighestCubeZ
  (bind _outactors (Actor|GetAllActorsOfClass "/Game/Blueprints/Game_Cube.Game_Cube_C"))
  (Variables|Default|SetHighestCube_ZValue 0.0)
  (for _array_element _outactors
    (if (> (.Z (Math|Vector|BreakVector (Transformation|GetWorldLocation (Variables|/Game/Blueprints/Game_Cube.Game_Cube_C|GetCube _array_element)))) (Variables|Default|GetHighestCube_ZValue))
      (Variables|Default|SetHighestCube_ZValue (.Z (Math|Vector|BreakVector (Transformation|GetWorldLocation (Variables|/Game/Blueprints/Game_Cube.Game_Cube_C|GetCube _array_element))))))))

(fn GetRandomSound
  (params (SoundArray :type Array%20of%20Sound%20Wave%20Object%20References))
  (return (Utilities|Array|Get(acopy) SoundArray (Math|Random|RandomInteger (Utilities|Array|Length SoundArray)))))