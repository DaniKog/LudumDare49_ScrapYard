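; Game cube actor that waits without gravity until released, then reports its hits and landing through event calls.
; After ReleaseCube, Tick waits out a cooldown, then signals landing when velocity nears zero, resetting the cooldown but leaving Released set.
; Every hit prints momentum; high-momentum hits on Floor-tagged actors trigger camera shake and a random soft impact sound.
; A hard-impact sound function exists but is not called here.
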(event EventBeginPlay)

(event Collision|EventActorBeginOverlap
  (params (OtherActor :type Actor%20Object%20Reference)))

(event EventTick
  (params (DeltaSeconds :type Float%20%28single-precision%29))
  (if (Variables|Default|GetReleased)
    (if (<= (Variables|Default|GetReleaseCoolDown) 0.0)
      (bind _returnvalue (Physics|GetPhysicsLinearVelocity (Variables|Default|GetCube) "None"))
      (if (Math|Float|NearlyEqual(Float) (Math|Vector|VectorLength _returnvalue) 0.0 (Variables|Default|GetVelocityTolorence))
        (Default|CallOnCubeLandeed)
        (Variables|Default|SetReleaseCoolDown 2.0))
      (else
        (Variables|Default|SetReleaseCoolDown (- (Variables|Default|GetReleaseCoolDown) DeltaSeconds))))))

(event Collision|EventHit
  (params (MyComp :type Primitive%20Component%20Object%20Reference) (Other :type Actor%20Object%20Reference) (OtherComp :type Primitive%20Component%20Object%20Reference) (bSelfMoved :type Boolean) (HitLocation :type Vector :default "0, 0, 0") (HitNormal :type Vector :default "0, 0, 0") (NormalImpulse :type Vector :default "0, 0, 0") (Hit :type Hit%20Result%20Structure%20%28by%20ref%29))
  (bind _cube (Variables|Default|GetCube))
  (Default|CallOnCubeHit)
  (bind _returnvalue (Physics|GetPhysicsLinearVelocity _cube "None"))
  (Development|PrintString (Utilities|String|ToString(Float) (* (Physics|GetMass _cube) (Math|Vector|VectorLength _returnvalue))) true true "(R=0.000000,G=0.660000,B=1.000000,A=1.000000)" (* (Physics|GetMass _cube) (Math|Vector|VectorLength _returnvalue)))
  (if (> (* (Physics|GetMass _cube) (Math|Vector|VectorLength _returnvalue)) 1.5e+03)
    (if (Actor|ActorHasTag Other "Floor")
      (Camera|PlayWorldCameraShake "/Game/Blueprints/FloorCamShake.FloorCamShake_C" (Camera|GetCameraLocation (Game|GetPlayerCameraManager 0)) 0.0 1e+02)
      (CallFunction|PlaySoftImpactSound))))

(fn ConstructionScript)

(fn ReleaseCube
  (Physics|SetEnableGravity (Variables|Default|GetCube) true)
  (Variables|Default|SetReleased true))

(fn PlayHardImpactSound
  (bind _hardimpact (Variables|Default|GetHardImpact))
  (bind _soundtoplay (CallFunction|GetRandomSound (Variables|Default|GetHardImpactSounds)))
  (if (Utilities|IsValid _soundtoplay)
    (Audio|Components|Audio|SetSound _hardimpact _soundtoplay)
    (Audio|Components|Audio|Play _hardimpact 0.0)))

(fn GetRandomSound
  (params (SoundArray :type Array%20of%20Sound%20Wave%20Object%20References))
  (return (Utilities|Array|Get(acopy) SoundArray (Math|Random|RandomInteger (Utilities|Array|Length SoundArray)))))

(fn PlaySoftImpactSound
  (bind _softimpact (Variables|Default|GetSoftImpact))
  (bind _soundtoplay (CallFunction|GetRandomSound (Variables|Default|GetSoftImpactSounds)))
  (if (Utilities|IsValid _soundtoplay)
    (Audio|Components|Audio|SetSound _softimpact _soundtoplay)
    (Audio|Components|Audio|Play _softimpact 0.0)))